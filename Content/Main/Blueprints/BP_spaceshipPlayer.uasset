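; Player spaceship pawn with flight controls, boost, twin lasers and a crosshair widget.
; Legacy axis inputs drive thrust and rotation, with turns auto-banking when roll input is idle, while Enhanced Input adds mouse steering.
; Boost changes max speed, Niagara thruster lifetime, FOV and camera lag.
; Holding fire loops a timer spawning projectiles from both muzzles, converging on a distant point deprojected from above screen center.
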(event `InputAxis|MoveForward`
  (params (AxisValue :type "Float (single-precision)"))
  (`self.AddMovementInput` (`self.GetActorForwardVector`) AxisValue))

(event `InputAxis|Turn`
  (params (AxisValue :type "Float (single-precision)"))
  (`self.K2_AddActorLocalRotation` (`KismetMathLibrary.MakeRotator` 0.0 0.0 (* AxisValue (`GameplayStatics.GetWorldDeltaSeconds`) 45.0)))
  (if (< (`KismetMathLibrary.Abs` (`self.RollInput`)) 0.1)
    (`self.K2_SetActorRotation` (`KismetMathLibrary.MakeRotator` (`KismetMathLibrary.FInterpTo` (.roll (`self.K2_GetActorRotation`)) (* AxisValue 20.0) (`GameplayStatics.GetWorldDeltaSeconds`) 5.0) (.pitch (`self.K2_GetActorRotation`)) (.yaw (`self.K2_GetActorRotation`))))))

(event `InputAxis|Roll`
  (params (AxisValue :type "Float (single-precision)"))
  (set `self.RollInput` AxisValue)
  (`self.K2_AddActorLocalRotation` (`KismetMathLibrary.MakeRotator` (* AxisValue (`GameplayStatics.GetWorldDeltaSeconds`) 180.0))))

(event `self.ReceiveBeginPlay`
  (bind _returnvalue (`|CreateWidget` "/Game/Widgets/WB_Crosshair.WB_Crosshair_C"))
  (`UserWidget.AddToViewport` _returnvalue 0)
  (`EnhancedInputSubsystemInterface.AddMappingContext` (pcsubsystem `EnhancedInputLocalPlayerSubsystem` (`GameplayStatics.GetPlayerController` 0)) "/Game/Main/IMC_Player.IMC_Player" 0 (struct)))

(event `InputAxis|Pitch`
  (params (AxisValue :type "Float (single-precision)"))
  (`self.K2_AddActorLocalRotation` (`KismetMathLibrary.MakeRotator` 0.0 (* AxisValue (`GameplayStatics.GetWorldDeltaSeconds`) 40.0))))

(event `EnhancedInput|/Game/Main/IA_Steer`
  (params (ActionValue :type "Vector2D Structure") (ElapsedSeconds :type "Float (double-precision)") (TriggeredSeconds :type "Float (double-precision)") (InputAction :type "InputAction Object Reference" :default "/Game/Main/IA_Steer.IA_Steer"))
  ; MouseSteeringYaw
  (:`Triggered`
    (`self.K2_AddActorLocalRotation` (`KismetMathLibrary.MakeRotator` 0.0 0.0 (* (`GameplayStatics.GetWorldDeltaSeconds`) (* (`KismetMathLibrary.BreakVector2D` ActionValue) (`self.MouseSensitivity`)) 1.0)))))

(event `EnhancedInput|/Game/Main/IA_Steer`
  (params (ActionValue :type "Vector2D Structure") (ElapsedSeconds :type "Float (double-precision)") (TriggeredSeconds :type "Float (double-precision)") (InputAction :type "InputAction Object Reference" :default "/Game/Main/IA_Steer.IA_Steer"))
  ; MouseSteeringPitch
  (:`Triggered`
    (`self.K2_AddActorLocalRotation` (`KismetMathLibrary.MakeRotator` 0.0 (* (`GameplayStatics.GetWorldDeltaSeconds`) (* (`.Y` (`KismetMathLibrary.BreakVector2D` ActionValue)) (`self.MouseSensitivity`)) 1.0)))))

(event `EnhancedInput|/Game/Main/IA_Boost`
  (params (ActionValue :type Boolean) (ElapsedSeconds :type "Float (double-precision)") (TriggeredSeconds :type "Float (double-precision)") (InputAction :type "InputAction Object Reference" :default "/Game/Main/IA_Boost.IA_Boost"))
  (:`Started`
    (set `FloatingPawnMovement.MaxSpeed` (`self.BoostSpeed`) (`self.FloatingPawnMovement`))
    (`NiagaraComponent.SetVariableFloat` (`self.NC_Thruster`) "User.ThrusterLifetime" 1.0)
    (`NiagaraComponent.SetVariableFloat` (`self.NC_Thruster_left`) "User.ThrusterLifetime" 1.0)
    (`NiagaraComponent.SetVariableFloat` (`self.NC_Thruster_right`) "User.ThrusterLifetime" 1.0)
    (`CameraComponent.SetFieldOfView` (`self.Camera`) 110.0)
    (set `SpringArmComponent.CameraLagSpeed` 4.0 (`self.SpringArm`)))
  (:`Completed`
    (set `FloatingPawnMovement.MaxSpeed` (`self.NormalSpeed`) (`self.FloatingPawnMovement`))
    (`NiagaraComponent.SetVariableFloat` (`self.NC_Thruster`) "User.ThrusterLifetime" 0.3)
    (`NiagaraComponent.SetVariableFloat` (`self.NC_Thruster_left`) "User.ThrusterLifetime" 0.3)
    (`NiagaraComponent.SetVariableFloat` (`self.NC_Thruster_right`) "User.ThrusterLifetime" 0.3)
    (`CameraComponent.SetFieldOfView` (`self.Camera`) 90.0)
    (set `SpringArmComponent.CameraLagSpeed` 8.0 (`self.SpringArm`))))

(event `InputAction|Fire`
  (params (Key :type "Key Structure"))
  ; Firing
  (:`Pressed`
    (bind _returnvalue (`KismetSystemLibrary.K2_SetTimerDelegate` (delegate `FireLaser`) 0.05 true))
    (set `self.FireTimerHandle` _returnvalue))
  (:`Released`
    (`KismetSystemLibrary.K2_ClearAndInvalidateTimerHandle` (`self.FireTimerHandle`))))

(event `FireLaser`
  (bind _returnvalue (`GameplayStatics.GetPlayerController` 0))
  (bind (_sizex _sizey) (`PlayerController.GetViewportSize` _returnvalue))
  (bind _returnvalue_2 (`SceneComponent.K2_GetComponentLocation` (`self.LaserMuzzle_Left`)))
  (bind _returnvalue_3 (`SceneComponent.K2_GetComponentLocation` (`self.LaserMuzzle_Right`)))
  (bind (_worldposition _worlddirection) (`GameplayStatics.DeprojectScreenToWorld` _returnvalue (`KismetMathLibrary.MakeVector2D` (* (`KismetMathLibrary.Conv_IntToDouble` _sizex) 0.5) (* (`KismetMathLibrary.Conv_IntToDouble` _sizey) 0.31))))
  ; Firing
  (set `self.AimPoint` (+ _worldposition (* _worlddirection (10000.0 10000.0 10000.0))))
  (`|SpawnActorFromClass` "/Game/Main/Blueprints/BP_LaserProjectile.BP_LaserProjectile_C" (`KismetMathLibrary.MakeTransform` _returnvalue_2 (`KismetMathLibrary.FindLookAtRotation` _returnvalue_2 (`self.AimPoint`))) "AlwaysSpawn" "MultiplyWithRoot" self null)
  (`|SpawnActorFromClass` "/Game/Main/Blueprints/BP_LaserProjectile.BP_LaserProjectile_C" (`KismetMathLibrary.MakeTransform` _returnvalue_3 (`KismetMathLibrary.FindLookAtRotation` _returnvalue_3 (`self.AimPoint`))) "AlwaysSpawn" "MultiplyWithRoot" self null))

(fn `UserConstructionScript`)